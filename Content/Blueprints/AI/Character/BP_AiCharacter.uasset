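; AI enemy character that, once possessed, periodically picks a random BP_Player, moves toward it and shoots at it.
; A looping move timer drives AIMoveTo until the target is within range, then a shooting timer fires through server and client events.
; Each shot turns to the target and line-traces with random spread to apply damage.
; Incoming damage goes to the health component; the death handler only casts the game state, and pawn sensing is unused.
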(event OnSeePawn(PawnSensing)
  (params (Pawn :type Pawn%20Object%20Reference)))

(event CharacterDeath(BP_AiHealthComponent)
  (Utilities|Casting|CastToBP_BaseGameState (Game|GetGameState)))

(event Custom|FindActor
  (bind _outactors (Actor|GetAllActorsOfClass "/Game/Blueprints/Player/BP_Player.BP_Player_C"))
  (Variables|Default|SetCharacter (Utilities|Array|Get(acopy) _outactors (Math|Random|RandomInteger (Utilities|Array|LastIndex _outactors))))
  (bind _returnvalue (Utilities|Time|SetTimerbyEvent (delegate Custom|Move) 0.01 true))
  (Variables|Default|SetMovingTimer _returnvalue))

(event Custom|Move
  (bind _movementresult (AI|AIMoveTo self (Transformation|GetActorLocation (Variables|Default|GetCharacter)) 0 1e+03 false)
    (:then
      (switch Utilities|FlowControl|Switch|SwitchonEPathFollowingResult _movementresult
        (:Success
          (Utilities|Time|ClearandInvalidateTimerbyHandle (Variables|Default|GetMovingTimer))
          (bind _returnvalue (Utilities|Time|SetTimerbyEvent (delegate Custom|Server_AiShooting) 0.1 true))
          (Variables|Default|SetShootingTimer _returnvalue))))))

(event Custom|Server_AiShooting
  (CallFunction|ClientAiShooting))

(event Custom|Client_AiShooting
  (CallFunction|StartShooting))

(event Game|Damage|EventAnyDamage
  (params (Damage :type Float%20%28single-precision%29) (DamageType :type Damage%20Type%20Object%20Reference) (InstigatedBy :type Controller%20Object%20Reference) (DamageCauser :type Actor%20Object%20Reference))
  (Default|ApplyDamage (Variables|Default|GetBP_AiHealthComponent) Damage))

(event EventPossessed
  (params (NewController :type Controller%20Object%20Reference))
  (Utilities|Time|SetTimerbyEvent (delegate Custom|FindActor) 5.0 true))

(fn ConstructionScript)

(fn StartShooting
  (bind _shootingrange (Variables|Default|GetShootingRange))
  (bind _shootingrange_2 (Variables|Default|GetShootingRange))
  (bind _returnvalue (* _shootingrange_2 -1.0))
  (bind _returnvalue_2 (Math|Random|RandomFloatinRange _returnvalue _shootingrange))
  (bind _character (Variables|Default|GetCharacter)
    (:then
      (Transformation|SetActorRotation (Math|Rotator|FindLookatRotation (Transformation|GetActorLocation) (Transformation|GetActorLocation _character)))
      (bind (_outhit _returnvalue_3) (Collision|LineTraceForObjects (Transformation|GetWorldLocation (Variables|Collision|GetCapsuleComponent)) (+ (Transformation|GetActorLocation (Variables|Default|GetCharacter)) (Math|Vector|MakeVector _returnvalue_2 _returnvalue_2 0.0)) (Utilities|Array|MakeArray "ObjectTypeQuery1" "ObjectTypeQuery3" "ObjectTypeQuery4") false 0 "ForDuration"))
      (if _returnvalue_3
        (Game|Damage|ApplyDamage (.HitActor (Collision|BreakHitResult _outhit)) 3.0 (Game|GetInstigatorController) self)))
    (:else)))