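; Health component for BP_Player that tracks damage and death.
; PlayerDamage subtracts damage, clamps Health at zero, then sets IsDead and reports victim and instigating controller to BP_BaseGM's CharacterDeath.
; The IsDead RepNotify fires the CharDead dispatcher and disables the owner's movement.
; Tick prints current Health on screen as a debug readout.
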(event EventBeginPlay
  (bind _asbp_player (Utilities|Casting|CastToBP_Player (Components|GetOwner)))
  (Variables|Default|SetCharacterOwner _asbp_player))

(event EventTick
  (params (DeltaSeconds :type Float%20%28single-precision%29))
  (Development|PrintString (Utilities|String|Append "Health: " (Utilities|String|ToString(Float) (Variables|Default|GetHealth))) true false "(R=0.000000,G=1.000000,B=0.412696,A=1.000000)" 0.0))

(fn PlayerDamage
  (params (Damage :type Float%20%28single-precision%29) (Instigator :type Controller%20Object%20Reference))
  (bind _output_get (Variables|Default|SetHealth (- (Variables|Default|GetHealth) Damage)))
  (bind _output_get_2 (Variables|Default|SetHealth (Math|Float|Max(Float) 0.0 _output_get)))
  (if (<= _output_get_2 0.0)
    (Variables|Default|SetIsDead true)
    (bind _asbp_base_gm (Utilities|Casting|CastToBP_BaseGM (Game|GetGameMode)))
    (Default|CharacterDeath _asbp_base_gm (Variables|Default|GetCharacterOwner) (.AsBP%20Player%20Controller (Utilities|Casting|CastToBP_PlayerController Instigator)))))

(fn OnRepIsDead
  (if (Variables|Default|GetIsDead)
    (Default|CallCharDead)
    (Pawn|Components|CharacterMovement|DisableMovement (Variables|/Script/Engine.Character|GetCharacterMovement (Variables|Default|GetCharacterOwner)))))