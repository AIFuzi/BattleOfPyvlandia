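; Player character with third-person and aim cameras, a weapon component and a health component.
; Aiming swaps to the FPS camera and scoped FPS mesh, hiding the body and weapon; spring arm length eases with movement and sprint.
; Fire and reload go through server events to the current weapon, while Tick updates look pitch.
; Damage feeds the health component; depletion destroys the actor and spawns a player at every PlayerStart.
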(event OnHealthEnded(BP_HealthComponent)
  (Development|PrintString "Health Ended")
  (Actor|DestroyActor)
  (bind _outactors (Actor|GetAllActorsOfClass "/Script/Engine.PlayerStart"))
  (for _array_element _outactors
    (Game|SpawnActorfromClass "BP_Player_C" (Math|Transform|MakeTransform (Transformation|GetActorLocation _array_element) "0,180.000000, 0" "1,1,1") "Undefined" 0 0)))

(event EventBeginPlay
  (Default|CreateWeapon (Variables|Default|GetBP_WeaponComponent) "/Game/Blueprints/Weapons/BP_Weapon.BP_Weapon_C")
  (CallFunction|TESTcreateScope "/Game/Blueprints/Weapons/BP_Scope.BP_Scope_C"))

(event Game|Damage|EventAnyDamage
  (params (Damage :type Float%20%28single-precision%29) (DamageType :type Damage%20Type%20Object%20Reference) (InstigatedBy :type Controller%20Object%20Reference) (DamageCauser :type Actor%20Object%20Reference))
  (Default|PlayerDamage (Variables|Default|GetBP_HealthComponent) Damage InstigatedBy))

(event EventPossessed
  (params (NewController :type Controller%20Object%20Reference))
  (Networking|SwitchHasAuthority))

(event EventTick
  (params (DeltaSeconds :type Float%20%28single-precision%29))
  (CallFunction|DynamicCameraMove)
  (CallFunction|SetLookAngle))

(event Input|ActionEvents|InputActionReload
  (params (Key :type Key%20Structure :default "None"))
  (:Pressed
    (CallFunction|ToggleAim false)
    (CallFunction|ServerReload)))

(event Input|ActionEvents|InputActionFire
  (params (Key :type Key%20Structure :default "None"))
  (:Pressed
    (CallFunction|ServerShoot true))
  (:Released
    (CallFunction|ServerShoot false)))

(event Input|MouseEvents|RightMouseButton
  (params (Key :type Key%20Structure :default "None"))
  (:Pressed
    (CallFunction|ToggleAim true))
  (:Released
    (CallFunction|ToggleAim false)))

(event Custom|Server_Shoot
  (params (UseWeapon :type Boolean))
  (bind _bp_weaponcomponent (Variables|Default|GetBP_WeaponComponent))
  (bind _currentweapon (Variables|/Script/BattleOfPyvlandia.WeaponComponent|GetCurrentWeapon _bp_weaponcomponent))
  (if UseWeapon
    (if (Class|WeaponActor|AbleforUseWeapon _currentweapon)
      (Class|WeaponActor|UseWeapon _currentweapon)
      (else
        (Class|WeaponActor|StopUseWeapon _currentweapon :!label _label)))
    (else
      (goto _label))))

(event Custom|Server_Reload
  (Class|WeaponActor|ReloadWeapon (Variables|/Script/BattleOfPyvlandia.WeaponComponent|GetCurrentWeapon (Variables|Default|GetBP_WeaponComponent))))

(fn ConstructionScript)

(fn DynamicCameraMove
  (bind _returnvalue (Utilities|Time|GetWorldDeltaSeconds))
  (bind _springarm (Variables|Default|GetSpringArm))
  (if (> (Math|Vector|VectorLength (Transformation|GetVelocity)) 0.0)
    (Variables|/Script/Engine.SpringArmComponent|SetTargetArmLength _springarm (Math|Interpolation|FInterpTo (Variables|/Script/Engine.SpringArmComponent|GetTargetArmLength (Variables|Default|GetSpringArm)) (Math|Float|SelectFloat 2.1e+02 1.9e+02 (Variables|Default|GetIsSprint)) _returnvalue 1e+01))
    (else
      (Variables|/Script/Engine.SpringArmComponent|SetTargetArmLength _springarm (Math|Interpolation|FInterpTo (Variables|/Script/Engine.SpringArmComponent|GetTargetArmLength (Variables|Default|GetSpringArm)) 1.5e+02 _returnvalue 1e+01)))))

(fn SetLookAngle
  (bind _returnvalue (Pawn|GetController))
  (Utilities|IsValid _returnvalue
    (:Is%20Valid
      (bind _output_get (Variables|Default|SetLookAngle (Transformation|GetActorForwardVector _returnvalue)))
      (Variables|Default|SetLookVerticaleAngle (.pitch (Math|Conversions|RotationFromXVector _output_get))))))

(fn ToggleAim
  (params (Aim :type Boolean))
  (bind _tps_camera (Variables|Default|GetTPS_Camera))
  (bind _bp_weaponcomponent (Variables|Default|GetBP_WeaponComponent))
  (bind _fps_camera (Variables|Default|GetFPS_Camera))
  (bind _mesh (Variables|Character|GetMesh))
  (bind _fps_mesh (Variables|Default|GetFPS_Mesh))
  (if Aim
    (Components|Activation|Deactivate _tps_camera)
    (Components|Activation|SetActive _fps_camera true false)
    (Development|SetHiddeninGame _mesh true false)
    (Development|SetHiddeninGame _fps_mesh false false)
    (bind _currentweapon (Variables|/Script/BattleOfPyvlandia.WeaponComponent|GetCurrentWeapon _bp_weaponcomponent)
      (:then
        (Rendering|SetActorHiddenInGame _currentweapon true)
        (|FindWeaponAttach_2)
        (Variables|Default|SetAiming true))
      (:else))
    (else
      (Components|Activation|Deactivate _fps_camera)
      (Components|Activation|SetActive _tps_camera true false)
      (Development|SetHiddeninGame _mesh false false)
      (Development|SetHiddeninGame _fps_mesh true false)
      (bind _currentweapon_2 (Variables|/Script/BattleOfPyvlandia.WeaponComponent|GetCurrentWeapon _bp_weaponcomponent)
        (:then
          (Rendering|SetActorHiddenInGame _currentweapon_2 false)
          (|UnhideWeapons_2)
          (Variables|Default|SetAiming false))
        (:else)))))

(fn TESTcreateScope
  (params (Class :type Actor%20Class%20Reference))
  (bind _returnvalue (Game|SpawnActorfromClass Class (Math|Transform|MakeTransform "0, 0, 0" "0, 0, 0" "1,1,1") "AlwaysSpawn" 0 0))
  (Transformation|AttachComponentToComponent _returnvalue (Variables|Default|GetFPS_Mesh) "Sk_Scope" "SnapToTarget" "SnapToTarget" "KeepRelative" true))