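; Spectator for the character customization screen that glides into a fixed view and shows the customization HUD.
; On BeginPlay, a fast looping timer eases location and rotation toward hard-coded targets, clearing itself once the controller is invalid.
; It also creates W_CustomizeHUD for its owning BP_PlayerController, stores it there as CustomHUD and adds it to the viewport.
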(event EventBeginPlay
  (bind _returnvalue (Utilities|Time|SetTimerbyFunctionName 0 "SetSpectatorLocation" 0.01 true))
  (Variables|Default|SetSetLocationTimer _returnvalue)
  (CallFunction|CreateCustomizeWidget))

(fn ConstructionScript)

(fn SetSpectatorLocation
  (Utilities|IsValid (Pawn|GetController)
    (:Is%20Valid
      (Transformation|SetActorLocation (Math|Interpolation|VInterpTo (Transformation|GetActorLocation) "-130.000000,510.000000,830.000000" (Utilities|Time|GetWorldDeltaSeconds) 1.0) false false)
      (Transformation|SetActorRotation (Math|Interpolation|RInterpTo (Transformation|GetActorRotation) "-40.000000,-90.000000, 0" (Utilities|Time|GetWorldDeltaSeconds) 1.0)))
    (:Is%20Not%20Valid
      (Utilities|Time|ClearandInvalidateTimerbyHandle (Variables|Default|GetSetLocationTimer)))))

(fn CreateCustomizeWidget
  (bind _returnvalue (Components|GetOwner))
  (Utilities|IsValid _returnvalue
    (:Is%20Valid
      (bind _asbp_player_controller (Utilities|Casting|CastToBP_PlayerController _returnvalue))
      (bind _returnvalue_2 (UserInterface|CreateWidget "/Game/UI/W_CustomizeHUD.W_CustomizeHUD_C" _asbp_player_controller))
      (Utilities|IsValid _returnvalue_2
        (:Is%20Valid
          (bind _output_get (Variables|/Game/Blueprints/Player/BP_PlayerController.BP_PlayerController_C|SetCustomHUD _asbp_player_controller _returnvalue_2))
          (UserInterface|Viewport|AddtoViewport _output_get 0))))))