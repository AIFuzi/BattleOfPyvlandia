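; BP_GameSpecator is a spectator pawn that shows a pre-start screen while the player looks and moves around.
; Input axes drive controller yaw and pitch, plus movement along the actor's forward, right and up vectors.
; BeginPlay creates the W_PreStart widget and adds it to the viewport.
; Unpossessing the pawn removes all widgets, not just the pre-start screen.
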(event EventBeginPlay
  (bind _returnvalue (UserInterface|CreateWidget "/Game/UI/PreStart/W_PreStart.W_PreStart_C"))
  (bind _output_get (Variables|Default|SetPreStartWidget _returnvalue))
  (Utilities|IsValid _output_get
    (:Is%20Valid
      (UserInterface|Viewport|AddtoViewport _returnvalue 0))))

(event EventUnpossessed
  (params (OldController :type Controller%20Object%20Reference))
  (Viewport|RemoveAllWidgets))

(event Input|AxisEvents|InputAxisTurn
  (params (AxisValue :type Float%20%28single-precision%29))
  (Pawn|Input|AddControllerYawInput AxisValue))

(event Input|AxisEvents|InputAxisLookUp
  (params (AxisValue :type Float%20%28single-precision%29))
  (Pawn|Input|AddControllerPitchInput AxisValue))

(event Input|AxisEvents|InputAxisMoveForward
  (params (AxisValue :type Float%20%28single-precision%29))
  (Pawn|Input|AddMovementInput (Transformation|GetActorForwardVector) AxisValue false))

(event Input|AxisEvents|InputAxisMoveRight
  (params (AxisValue :type Float%20%28single-precision%29))
  (Pawn|Input|AddMovementInput (Transformation|GetActorRightVector) AxisValue false))

(event Input|AxisEvents|InputAxisSpectatorUp
  (params (AxisValue :type Float%20%28single-precision%29))
  (Pawn|Input|AddMovementInput (Transformation|GetActorUpVector) AxisValue false))

(fn ConstructionScript)