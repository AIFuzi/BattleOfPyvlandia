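; Game state that runs the pre-match countdown, match clock and Red/Blue team points.
; On the server, Tick starts a looping one-second countdown once enough players join, and resets the round flag and start-time value while below that count.
; When the countdown expires, it calls StartGame on BP_BaseGM and starts a GameTick timer that advances the minute and second values exposed by GetGameTime.
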(event EventTick
  (params (DeltaSeconds :type Float%20%28single-precision%29))
  (Networking|SwitchHasAuthority
    (:Authority
      (if (>= (Utilities|Array|Length (Variables|Default|GetPlayerArray)) (Variables|PreStartGame|GetPlayerForStartGame))
        (if (not (Variables|PreStartGame|GetRoundStarted))
          (Variables|PreStartGame|SetRoundStarted true)
          (bind _returnvalue (Utilities|Time|SetTimerbyFunctionName 0 "RoundStartTime" 1.0 true))
          (Variables|PreStartGame|SetStartGameTimer _returnvalue))
        (else
          (Variables|PreStartGame|SetRoundStarted false)
          (Variables|PreStartGame|SetTimeForStarGame (.TimeForStarGame (Utilities|GetClassDefaults (Utilities|GetClass self)))))))))

(event EventBeginPlay
  (Variables|PreStartGame|SetTimeForStart (Math|Timespan|MakeTimespan 0 0 0 (Variables|PreStartGame|GetTimeForStarGame) 0)))

(fn ConstructionScript)

(fn SetStartGame)

(fn RoundStartTime
  (bind _output_get (Variables|PreStartGame|SetTimeForStart (- (Variables|PreStartGame|GetTimeForStart) (Class|KismetMathLibrary|MakeTimespan2 0 0 0 1))))
  (bind _output_get_2 (Variables|PreStartGame|SetTimeForStarGame (.Seconds (Class|KismetMathLibrary|BreakTimespan2 _output_get))))
  (if (<= _output_get_2 0)
    (Utilities|Time|ClearandInvalidateTimerbyHandle (Variables|PreStartGame|GetStartGameTimer))
    (bind _asbp_base_gm (Utilities|Casting|CastToBP_BaseGM (Game|GetGameMode)))
    (Default|StartGame _asbp_base_gm)
    (Utilities|Time|SetTimerbyFunctionName 0 "GameTick" 1.0 true)))

(fn StartTick
  (Variables|PreStartGame|SetTimeForStarGame (- (Variables|PreStartGame|GetTimeForStarGame) 1)))

(fn GameTick
  (bind _output_get (Variables|Game|SetTimeGame (+ (Variables|Game|GetTimeGame) (Math|Timespan|MakeTimespan 0 0 0 1))))
  (bind _output_get_2 (Variables|Game|SetGameSeconds (.Seconds (Math|Timespan|BreakTimespan _output_get))))
  (if (>= _output_get_2 59)
    (Variables|Game|SetGameSeconds 0)
    (bind _output_get_3 (Variables|Game|SetTimeGame (+ (Variables|Game|GetTimeGame) (Math|Timespan|MakeTimespan 0 0 1))))
    (Variables|Game|SetGameMinute (.Minutes (Math|Timespan|BreakTimespan _output_get_3)))))

(fn GetGameTime
  (return (Variables|Game|GetGameMinute) (Variables|Game|GetGameSeconds)))

(fn AddPoints
  (params (RedPoints :type Integer) (BluePoints :type Integer))
  (Variables|Points|SetRedPoint (+ (Variables|Points|GetRedPoint) RedPoints))
  (Variables|Points|SetBluePoints (+ (Variables|Points|GetBluePoints) BluePoints)))