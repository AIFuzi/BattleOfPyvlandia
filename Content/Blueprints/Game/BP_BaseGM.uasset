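; Base game mode that handles player death, spectating and respawn placement.
; CharacterDeath announces the death, starts the player controller's respawn delay, then has that controller possess a newly spawned character-customization spectator.
; SpawnPlayer picks a random entry from the BP_PlayerStart actors reporting free and delegates spawning to it.
; A separate SpawnSpectator function, not called here, possesses a game spectator at the controlled pawn's transform.
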(fn ConstructionScript)

(fn CharacterDeath
  (params (Death%20player :type BP%20Player%20Object%20Reference) (Dealth%20instigator :type BP%20Player%20Controller%20Object%20Reference))
  (Default|CallPlayerDead Death%20player Dealth%20instigator)
  (bind _asbp_player_controller (Utilities|Casting|CastToBP_PlayerController (Pawn|GetController Death%20player)))
  (Utilities|FlowControl|Sequence
    (:then_0
      (Default|RespawnDelayStart _asbp_player_controller (Variables|Default|GetRespawnTime)))
    (:then_1
      (CallFunction|PossesonCustomezeSpectator Death%20player _asbp_player_controller))))

(fn SpawnPlayer
  (params (Player :type BP%20Player%20Controller%20Object%20Reference))
  (bind _freespawn (CallFunction|GetFreeSpawn))
  (bind _output_get (LocalVariables|SetL_PlayerStart (Utilities|Array|Get(acopy) _freespawn (Math|Random|RandomInteger (Utilities|Array|LastIndex _freespawn)))))
  (Default|SpawnPlayer _output_get Player))

(fn GetFreeSpawn
  (bind _outactors (Actor|GetAllActorsOfClass "/Game/Blueprints/Game/BP_PlayerStart.BP_PlayerStart_C"))
  (for _array_element _outactors
    (if (Default|IsFree _array_element)
      (Utilities|Array|Add (LocalVariables|GetL_FreeSpawn) _array_element)))
  (return (LocalVariables|GetL_FreeSpawn)))

(fn SpawnSpectator
  (params (Player :type BP%20Player%20Object%20Reference) (DeathInstigator :type BP%20Player%20Controller%20Object%20Reference))
  (bind _returnvalue (Game|SpawnActorfromClass "/Game/Blueprints/Game/Spectator/BP_GameSpecator.BP_GameSpecator_C" (Transformation|GetActorTransform (Pawn|GetControlledPawn DeathInstigator)) "AlwaysSpawn" 0 0))
  (bind _output_get (Variables|Default|SetSpectator _returnvalue))
  (Pawn|Possess DeathInstigator _output_get))

(fn PossesonCustomezeSpectator
  (params (Player :type BP%20Player%20Object%20Reference) (DeathInstigator :type BP%20Player%20Controller%20Object%20Reference))
  (bind _outactors (Actor|GetAllActorsOfClass "/Game/Blueprints/Game/Spectator/BP_CustomizeCharacterSpectator.BP_CustomizeCharacterSpectator_C"))
  (bind _returnvalue (Game|SpawnActorfromClass "/Game/Blueprints/Game/Spectator/BP_CustomizeCharacterSpectator.BP_CustomizeCharacterSpectator_C" (Transformation|GetActorTransform DeathInstigator) "AlwaysSpawn" 0 0))
  (Pawn|Possess DeathInstigator _returnvalue))