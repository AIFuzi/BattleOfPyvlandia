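; BP_PlayerStart is a spawn point that creates and possesses player characters and reports whether it is occupied.
; SpawnPlayer always spawns a BP_Player at the actor's transform regardless of collision, has the given controller possess it, and records it as the occupant.
; Capsule overlaps track a single BP_Player reference, cleared when that character leaves.
; IsFree returns true when that reference is not valid.
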(event OnComponentEndOverlap(CapsuleComponent)
  (params (OverlappedComponent :type Primitive%20Component%20Object%20Reference) (OtherActor :type Actor%20Object%20Reference) (OtherComp :type Primitive%20Component%20Object%20Reference) (OtherBodyIndex :type Integer))
  (if (== OtherActor (Variables|Default|GetCharacteInside))
    (Variables|Default|SetCharacteInside 0)))

(event OnComponentBeginOverlap(CapsuleComponent)
  (params (OverlappedComponent :type Primitive%20Component%20Object%20Reference) (OtherActor :type Actor%20Object%20Reference) (OtherComp :type Primitive%20Component%20Object%20Reference) (OtherBodyIndex :type Integer) (bFromSweep :type Boolean) (SweepResult :type Hit%20Result%20Structure%20%28by%20ref%29))
  (bind _asbp_player (Utilities|Casting|CastToBP_Player OtherActor))
  (Variables|Default|SetCharacteInside _asbp_player))

(fn ConstructionScript)

(fn SpawnPlayer
  (params (Player :type BP%20Player%20Controller%20Object%20Reference))
  (bind _returnvalue (Game|SpawnActorfromClass "/Game/Blueprints/Player/BP_Player.BP_Player_C" (Transformation|GetActorTransform) "AlwaysSpawn" Player 0))
  (bind _output_get (Variables|Default|SetCharacteInside _returnvalue))
  (Pawn|Possess Player _output_get)
  (return (Variables|Default|GetCharacteInside)))

(fn IsFree
  (Utilities|IsValid (Variables|Default|GetCharacteInside)
    (:Is%20Valid
      (return false))
    (:Is%20Not%20Valid
      (return true))))