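; Weapon Blueprint that adds camera recoil when the weapon effect plays and passes ammo counts to the player controller.
; BeginPlay caches the weapon owner and binds the effect delegate to a client event that runs the SetRecoil timeline.
; The timeline curve, scaled by recoil strength and negated, feeds the owner's controller pitch input.
; Tick copies current and total ammo into BP_PlayerController whenever GetOwner casts to it.
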(event Custom|OnPlayWeaponEffect_Event_0
  (CallFunction|ClientPlayWeaponEffect))

(event Custom|Client_PlayWeaponEffect
  (bind _recoil (Timeline|SetRecoil PlayFromStart)
    (:Update
      (bind _recoilower (Variables|Default|GetRecoilOwer)
        (:then
          (Pawn|Input|AddControllerPitchInput _recoilower (* _recoil (Variables|Default|GetRecoilStrenght) -1.0)))
        (:else)))))

(event EventTick
  (params (DeltaSeconds :type Float%20%28single-precision%29))
  (bind _asbp_player_controller (Utilities|Casting|CastToBP_PlayerController (Components|GetOwner)))
  (Variables|/Game/Blueprints/Player/BP_PlayerController.BP_PlayerController_C|SetCurrent _asbp_player_controller (Variables|Default|GetCurrentAmmo))
  (Variables|/Game/Blueprints/Player/BP_PlayerController.BP_PlayerController_C|SetTotal _asbp_player_controller (Variables|Default|GetTotalAmmo)))

(event EventBeginPlay
  (EventDispatchers|AssignOnPlayWeaponEffect (delegate Custom|OnPlayWeaponEffect_Event_0))
  (Variables|Default|SetRecoilOwer (Variables|Default|GetWeaponOwner)))

(fn ConstructionScript)