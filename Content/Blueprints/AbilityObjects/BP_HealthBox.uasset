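; BP_HealthBox is a health pickup item that heals the player who uses it.
; UseItem adds a fixed amount to the player's BPHealthComponent Health, but only when Health is below a threshold.
; After healing, the box destroys itself only if its OverlapedActors array holds more than two entries.
; The event graph is inactive, so all logic of its own lives in UseItem.
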(event EventBeginPlay
  (|CallParentFunction) ; This node is disabled and will not be called.\nDrag off pins to build functionality.
)

(event Collision|EventActorBeginOverlap
  (params (OtherActor :type Actor%20Object%20Reference)))

(event EventTick
  (params (DeltaSeconds :type Float%20%28single-precision%29))
  (|CallParentFunction DeltaSeconds) ; This node is disabled and will not be called.\nDrag off pins to build functionality.
)

(fn ConstructionScript
  (|CallParentFunction))

(fn UseItem
  (params (Player :type BP%20Player%20Object%20Reference))
  (LocalVariables|SetL_Player Player)
  (if (< (Variables|/Script/BattleOfPyvlandia.HealthComponent|GetHealth (Variables|/Game/Blueprints/Player/BP_Player.BP_Player_C|GetBP_HealthComponent (LocalVariables|GetL_Player))) 6e+01)
    (Variables|/Script/BattleOfPyvlandia.HealthComponent|SetHealth (Variables|/Game/Blueprints/Player/BP_Player.BP_Player_C|GetBP_HealthComponent (LocalVariables|GetL_Player)) (+ (Variables|/Script/BattleOfPyvlandia.HealthComponent|GetHealth (Variables|/Game/Blueprints/Player/BP_Player.BP_Player_C|GetBP_HealthComponent (LocalVariables|GetL_Player))) 4e+01))
    (if (> (Utilities|Array|Length (Variables|Default|GetOverlapedActors)) 2)
      (Actor|DestroyActor))))