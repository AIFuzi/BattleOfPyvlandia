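; BP_Grenade is a timed grenade actor that explodes a few seconds after spawning.
; BeginPlay sets a timer for the Explosion function, which applies radial damage credited to the instigator controller and destroys the actor.
; The Destroyed event passes the actor's location through Server_SpawnEffect to Client_SpawnEffect, which spawns the explosion particle effect.
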(event Custom|Client_SpawnEffect
  (params (Location :type Vector))
  (Effects|SpawnEmitteratLocation "/Game/Assets/StarterContent/Particles/P_Explosion.P_Explosion" Location))

(event Custom|Server_SpawnEffect
  (params (Location :type Vector))
  (CallFunction|ClientSpawnEffect Location))

(event EventBeginPlay
  (|CallParentFunction)
  (Utilities|Time|SetTimerbyFunctionName 0 "Explosion" 5.0))

(event EventDestroyed
  (CallFunction|ServerSpawnEffect (Transformation|GetActorLocation)))

(fn ConstructionScript
  (|CallParentFunction))

(fn Explosion
  (Game|Damage|ApplyRadialDamage 1.3e+02 (Transformation|GetActorLocation) 5e+02 0 0 self (Game|GetInstigatorController) false "ECC_Visibility")
  (Actor|DestroyActor))