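; BP_AmmoBox is an ammo pickup that adds ammo to the current weapon of a BP_Player overlapping its Box1 component.
; CheckForItemItem records players in OverlapedActors and passes them to UseItem, which grants the ammo and destroys the box once over two players are recorded.
; The repeat check compares against each entry separately, so it blocks a returning player only while they are the sole entry.
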(event OnComponentBeginOverlap(Box)
  (params (OverlappedComponent :type Primitive%20Component%20Object%20Reference) (OtherActor :type Actor%20Object%20Reference) (OtherComp :type Primitive%20Component%20Object%20Reference) (OtherBodyIndex :type Integer) (bFromSweep :type Boolean) (SweepResult :type Hit%20Result%20Structure%20%28by%20ref%29)))

(event OnComponentBeginOverlap(Box1)
  (params (OverlappedComponent :type Primitive%20Component%20Object%20Reference) (OtherActor :type Actor%20Object%20Reference) (OtherComp :type Primitive%20Component%20Object%20Reference) (OtherBodyIndex :type Integer) (bFromSweep :type Boolean) (SweepResult :type Hit%20Result%20Structure%20%28by%20ref%29))
  (CallFunction|CheckforItemItem OtherActor))

(fn ConstructionScript
  (|CallParentFunction))

(fn CheckforItemItem
  (params (OverlapActor :type Actor%20Object%20Reference))
  (LocalVariables|SetL_OverlapActor OverlapActor)
  (if (<= (Utilities|Array|Length (Variables|Default|GetOverlapedActors)) 0)
    (bind _asbp_player (Utilities|Casting|CastToBP_Player (LocalVariables|GetL_OverlapActor)))
    (bind _output_get (LocalVariables|SetL_Player _asbp_player))
    (Utilities|Array|AddUnique (Variables|Default|GetOverlapedActors) _output_get)
    (CallFunction|UseItem (LocalVariables|GetL_Player))
    (else
      (for _array_element (Variables|Default|GetOverlapedActors)
        (if (!= _array_element (LocalVariables|GetL_OverlapActor))
          (bind _asbp_player_2 (Utilities|Casting|CastToBP_Player (LocalVariables|GetL_OverlapActor)))
          (bind _output_get_2 (LocalVariables|SetL_Player _asbp_player_2))
          (Utilities|Array|AddUnique (Variables|Default|GetOverlapedActors) _output_get_2)))
      (bind _l_player (LocalVariables|GetL_Player)
        (:then
          (CallFunction|UseItem _l_player))
        (:else)))))

(fn UseItem
  (params (Player :type BP%20Player%20Object%20Reference))
  (bind _currentweapon (Variables|/Script/BattleOfPyvlandia.WeaponComponent|GetCurrentWeapon (Variables|/Game/Blueprints/Player/BP_Player.BP_Player_C|GetBP_WeaponComponent Player))
    (:then
      (Variables|/Script/BattleOfPyvlandia.WeaponActor|SetTotalAmmo _currentweapon (+ (Variables|/Script/BattleOfPyvlandia.WeaponActor|GetTotalAmmo _currentweapon) 30))
      (if (> (Utilities|Array|Length (Variables|Default|GetOverlapedActors)) 2)
        (Actor|DestroyActor)))
    (:else)))