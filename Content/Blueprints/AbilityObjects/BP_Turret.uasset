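; Deployable turret actor that snaps to the ground below on spawn, or destroys itself if none is found.
; Its radius sphere lists overlapping actors not in the friendly class list, running looping timers while any remain.
; These timers yaw toward the first listed actor and fire forward line traces that damage whatever they hit.
; Damage depletes its health until destruction spawns an explosion; Tick draws debug range and target info.
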(event OnComponentBeginOverlap(TurretRadiusSphere)
  (params (OverlappedComponent :type Primitive%20Component%20Object%20Reference) (OtherActor :type Actor%20Object%20Reference) (OtherComp :type Primitive%20Component%20Object%20Reference) (OtherBodyIndex :type Integer) (bFromSweep :type Boolean) (SweepResult :type Hit%20Result%20Structure%20%28by%20ref%29))
  (bind _actoradd (CallFunction|SetEnemy OtherActor))
  (Utilities|IsValid _actoradd
    (:Is%20Valid
      (Utilities|Array|AddUnique (Variables|Default|GetOverlapedActors) _actoradd)
      (bind _returnvalue (Utilities|Time|SetTimerbyFunctionName 0 "RotateToEnemy" (Variables|TurretOptions|GetRotateSpeed) true))
      (Variables|Default|SetRotateToEnemyTimer _returnvalue)
      (bind _returnvalue_2 (Utilities|Time|SetTimerbyFunctionName 0 "ShootToEnemy" (Variables|TurretOptions|GetShootingSpeed) true))
      (Variables|Default|SetShootingTimer _returnvalue_2))))

(event OnComponentEndOverlap(TurretRadiusSphere)
  (params (OverlappedComponent :type Primitive%20Component%20Object%20Reference) (OtherActor :type Actor%20Object%20Reference) (OtherComp :type Primitive%20Component%20Object%20Reference) (OtherBodyIndex :type Integer))
  (Utilities|Array|RemoveItem (Variables|Default|GetOverlapedActors) OtherActor)
  (if (not (> (Utilities|Array|Length (Variables|Default|GetOverlapedActors)) 0))
    (Utilities|Time|ClearandInvalidateTimerbyHandle (Variables|Default|GetRotateToEnemyTimer))
    (Utilities|Time|ClearandInvalidateTimerbyHandle (Variables|Default|GetShootingTimer))))

(event Game|Damage|EventAnyDamage
  (params (Damage :type Float%20%28single-precision%29) (DamageType :type Damage%20Type%20Object%20Reference) (InstigatedBy :type Controller%20Object%20Reference) (DamageCauser :type Actor%20Object%20Reference))
  (Variables|TurretOptions|SetTurretHealth (- (Variables|TurretOptions|GetTurretHealth) Damage))
  (bind _output_get (Variables|TurretOptions|SetTurretHealth (Math|Float|Max(Float) (Variables|TurretOptions|GetTurretHealth) 0.0)))
  (if (<= _output_get 0.0)
    (Actor|DestroyActor)))

(event EventDestroyed
  (Effects|SpawnEmitteratLocation "/Game/Assets/StarterContent/Particles/P_Explosion.P_Explosion" (Transformation|GetActorLocation)))

(event EventBeginPlay
  (bind _returnvalue (Transformation|GetActorLocation))
  (bind (_outhit _returnvalue_2) (Collision|LineTraceByChannel _returnvalue (- _returnvalue "0, 0,150.000000") "TraceTypeQuery1" false 0 "None"))
  (if _returnvalue_2
    (Transformation|SetActorLocation (.Location (Collision|BreakHitResult _outhit)) false false)
    (else
      (Actor|DestroyActor))))

(event EventTick
  (params (DeltaSeconds :type Float%20%28single-precision%29))
  (bind _returnvalue (Transformation|GetActorLocation))
  (Class|KismetSystemLibrary|DrawDebugCylinder _returnvalue (+ _returnvalue "0, 0,40.000000") (Components|Sphere|GetScaledSphereRadius (Variables|Default|GetTurretRadiusSphere)) 12 "(R=1.000000,G=0.329114,B=0.000000,A=1.000000)" 0.0 0.0)
  (for _array_element (Variables|Default|GetOverlapedActors)
    (Development|PrintString (Utilities|String|Append "Overlaped list: " (Utilities|GetDisplayName _array_element)) true true "(R=1.000000,G=0.535740,B=0.000000,A=1.000000)" 0.0)))

(fn ConstructionScript)

(fn RotatetoEnemy
  (bind _returnvalue (Transformation|GetActorRotation))
  (Transformation|SetActorRotation (Math|Interpolation|RInterpTo (Transformation|GetActorRotation) (Math|Rotator|MakeRotator (.roll _returnvalue) (.pitch _returnvalue) (.yaw (Math|Rotator|FindLookatRotation (Transformation|GetActorLocation) (Transformation|GetActorLocation (Utilities|Array|Get(acopy) (Variables|Default|GetOverlapedActors)))))) (Utilities|Time|GetWorldDeltaSeconds) 1.0)))

(fn ShoottoEnemy
  (bind _sphere (Variables|Default|GetSphere))
  (bind _returnvalue (Transformation|GetWorldLocation _sphere))
  (bind (_outhit _returnvalue_2) (Collision|LineTraceForObjects _returnvalue (+ _returnvalue (* (Math|Vector|GetForwardVector _sphere) 1e+03)) (Utilities|Array|MakeArray "ObjectTypeQuery1" "ObjectTypeQuery3" "ObjectTypeQuery4") false (Utilities|Array|MakeArray self) "None"))
  (if _returnvalue_2
    (Game|Damage|ApplyPointDamage (.HitActor (Collision|BreakHitResult _outhit)) 3.0 (.Location (Collision|BreakHitResult _outhit)) _outhit (Game|GetInstigatorController) self)))

(fn SetEnemy
  (params (Actor :type Actor%20Object%20Reference))
  (bind _output_get (LocalVariables|SetL_Actor Actor))
  (for _array_element (Variables|TurretOptions|GetFrendlyList)
    (if (!= _array_element (Utilities|GetClass _output_get))
      (LocalVariables|SetL_Actor _output_get)
      (else
        (LocalVariables|SetL_Actor 0))))
  (return (LocalVariables|GetL_Actor)))